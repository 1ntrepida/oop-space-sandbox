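; A sphere actor that circles along a horizontal path and has keyboard controls for its spin rate.
; Each Tick steps Theta by a fixed, frame-rate-dependent amount, adds its sine and cosine as a world offset, and applies a local yaw rotation.
; N, M and X lower, raise and zero RotationSpeedConstant, but its visible link to DeltaSeconds sits in unexecuted nodes, leaving the yaw source unresolved.
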(event EventTick
  (params (DeltaSeconds :type Float%20%28single-precision%29))
  (Variables|Default|SetdeltaSeconds DeltaSeconds)
  ;[1 1 1] The sphere's orbit
  (bind _output_get (Variables|Default|SetTheta (+ (Variables|Default|GetTheta) 0.5)))
  (Transformation|AddWorldOffset (Variables|Default|GetDefaultSceneRoot) (Math|Vector|MakeVector (Math|Trig|Sin(Degrees) _output_get) (Math|Trig|Cos(Degrees) _output_get) 0.0) false false)
  ;[1 1 1] The sphere's rotation
  (Transformation|AddActorLocalRotation (Math|Rotator|MakeRotator 0.0 0.0 (stale _result)) false false))

(event EventBeginPlay
  ;[1 1 1] Enable Keyboard Input
  (Input|EnableInput (Game|GetPlayerController 0)))

(event Input|KeyboardEvents|M
  (params (Key :type Key%20Structure :default "AnyKey"))
  ;[1 1 1] Increase Spin Rate
  (:Pressed
    (Variables|Default|SetRotationSpeedConstant (+ (Variables|Default|GetRotationSpeedConstant) 1.0))))

(event Input|KeyboardEvents|N
  (params (Key :type Key%20Structure :default "AnyKey"))
  ;[1 1 1] Decreases Rotation Rate
  (:Pressed
    (Variables|Default|SetRotationSpeedConstant (+ (Variables|Default|GetRotationSpeedConstant) -1.0))))

(event Input|KeyboardEvents|X
  (params (Key :type Key%20Structure :default "AnyKey"))
  ;[1 1 1] Resets Rotation Rate
  (:Pressed
    (Variables|Default|SetRotationSpeedConstant 0.0)))

(fn ConstructionScript)