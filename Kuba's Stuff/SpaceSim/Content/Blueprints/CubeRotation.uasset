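; CubeRotation is an actor Blueprint for a spinning cube whose spin rate the player adjusts from the keyboard.
; BeginPlay enables input from the first player controller, and Tick applies a local yaw rotation each frame.
; M raises the Yawchange variable, N lowers it and X resets it to zero.
; Tick adds DeltaSeconds to Yawchange rather than multiplying, so spin depends on frame rate and a slow drift remains after reset.
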(event EventTick
  (params (DeltaSeconds :type Float%20%28single-precision%29))
  ;[1 1 1] Starts the cube's rotation
  (Transformation|AddActorLocalRotation (Math|Rotator|MakeRotator 0.0 0.0 (+ DeltaSeconds (Variables|Default|Getyawchange))) false false))

(event EventBeginPlay
  ;[1 1 1] Enables Keyboard Input
  (Input|EnableInput (Game|GetPlayerController 0)))

(event Input|KeyboardEvents|M
  (params (Key :type Key%20Structure :default "AnyKey"))
  ;[1 1 1] Increase Spin Rate
  (:Pressed
    (Variables|Default|Setyawchange (+ (Variables|Default|Getyawchange) 1.0))))

(event Input|KeyboardEvents|N
  (params (Key :type Key%20Structure :default "AnyKey"))
  ;[1 1 1] Decreases Spin Rate
  (:Pressed
    (Variables|Default|Setyawchange (+ (Variables|Default|Getyawchange) -1.0))))

(event Input|KeyboardEvents|X
  (params (Key :type Key%20Structure :default "AnyKey"))
  ;[1 1 1] Resets Spin Rate
  (:Pressed
    (Variables|Default|Setyawchange 0.0)))

(fn ConstructionScript)